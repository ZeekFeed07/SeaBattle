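; BP_MenuPawn is the main menu pawn for SeaBattle, setting up the menu interface when play begins.
; InitUI creates WBP_MainMenu, stores it, adds it to the viewport, and switches the player controller to UI-only input with a visible cursor.
; It binds an event to the widget's open-clicked callback, and its OpenLevel function loads L_MainGameplay.
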(event `self.ReceiveBeginPlay`
  (`|ExecutionSequence`
    (:`then_0`
      (`self.InitUI`))))

(fn `GetInterfaceRef`
  (returns (InterfaceRef :type "/Game/SeaBattle/Dev/UI/MainMenu/WBP_MainMenuBase Object Reference"))
  (return (`self.InterfaceRef`)))

(fn `InitUI`
  (bind _returnvalue (`GameplayStatics.GetPlayerController` 0))
  (`|ExecutionSequence`
    (:`then_0`
      (bind _returnvalue_2 (`|CreateWidget` "/Game/SeaBattle/Dev/UI/MainMenu/WBP_MainMenu.WBP_MainMenu_C"))
      (`self.SetInterfaceRef` _returnvalue_2))
    (:`then_1`
      (`WidgetBlueprintLibrary.SetInputMode_UIOnlyEx` _returnvalue null)
      (set `PlayerController.bShowMouseCursor` true _returnvalue))
    (:`then_2`
      (add `/Game/SeaBattle/Dev/UI/MainMenu/WBP_MainMenuBase.OnOpenClicked` (`self.InterfaceRef`) (`|CreateDelegate` :!event `OpenLevel`)))))

(fn `OpenLevel`
  (`GameplayStatics.OpenLevelBySoftObjectPtr` "/Game/SeaBattle/Maps/L_MainGameplay.L_MainGameplay")
  (return))

(fn `SetInterfaceRef`
  (params (`New Interface Ref` :type "/Game/SeaBattle/Dev/UI/MainMenu/WBP_MainMenuBase Object Reference (by ref)"))
  (bind _output_get (set `self.InterfaceRef` `New Interface Ref`))
  (`UserWidget.AddToViewport` _output_get 0)
  (return))

(fn `UserConstructionScript`)