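; Player controller for the Sea Battle ship setup phase, where the player places, rotates, removes and deletes ships on the grid.
; On BeginPlay it spawns BP_GameManager, binds the HUD's ship size buttons and enables the mouse cursor.
; It swaps Enhanced Input mapping contexts between editing and placing modes.
; While placing, a looping timer traces under the cursor, moving the ship to the hovered sea cell and recoloring surrounding cells.
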(event `self.ReceiveTick`
  (params (DeltaSeconds :type "Float (single-precision)"))
  ;[0.001 0.001 0.001 1 32] Tick
)

(event `self.ReceiveBeginPlay`
  ;[0.001 0.001 0.001 1 32] BeginPlay
  (`|ExecutionSequence`
    (:`then_0`
      (`self.StartInitialize`))
    (:`then_1`
      (`self.SetShipEditingMode`))))

(event `OnSizeClicked`
  (params (ShipSize :type "EShipLength Enum" :default "ONE"))
  (`self.MainManager`
    (:`then`
      (`|ExecutionSequence`
        (:`then_0`
          (`self.SetShipPlacingMode`))
        (:`then_1`
          (bind _returnvalue (`KismetSystemLibrary.K2_SetTimerDelegate` (`|CreateDelegate` :!event `OnMousePositionChange`) 0.01 true true))
          (set `self.MouseFollowTimer` _returnvalue))))
    (:`else`
      (`KismetSystemLibrary.PrintString` "Error: GameManager is not valid. (BP_MainPlayerController | OnSizeClicked)"))))

(event `EnhancedInput|/Game/SeaBattle/Dev/Input/Actions/IA_PlaceShip`
  (params (ActionValue :type Boolean) (ElapsedSeconds :type "Float (double-precision)") (TriggeredSeconds :type "Float (double-precision)") (InputAction :type "InputAction Object Reference" :default "/Game/SeaBattle/Dev/Input/Actions/IA_PlaceShip.IA_PlaceShip"))
  (:`Completed`
    (bind _mainmanager (`self.MainManager`)
      (:`then`
        (bind _issuccessful (`/Game/SeaBattle/Dev/Core/BP_GameManager.PlaceShipToField` _mainmanager (`self.LastCellID`)))
        (if _issuccessful
          (`KismetSystemLibrary.K2_ClearAndInvalidateTimerHandle` (`self.MouseFollowTimer`))
          (`self.SetShipEditingMode`)))
      (:`else`
        (`KismetSystemLibrary.PrintString` "Error: GameManager is not valid. (BP_MainPlayerController | IA_PlaceShip)")))))

(event `OnMousePositionChange`
  (`self.MoveShipToMouse`))

(event `EnhancedInput|/Game/SeaBattle/Dev/Input/Actions/IA_RemoveShip`
  (params (ActionValue :type Boolean) (ElapsedSeconds :type "Float (double-precision)") (TriggeredSeconds :type "Float (double-precision)") (InputAction :type "InputAction Object Reference" :default "/Game/SeaBattle/Dev/Input/Actions/IA_RemoveShip.IA_RemoveShip"))
  (bind (_locationx _locationy) (`self.GetMousePosition`))
  (bind (_worldlocation _worlddirection) (`self.DeprojectScreenPositionToWorld` _locationx _locationy))
  (:`Completed`
    (bind (_outhit _returnvalue) (`KismetSystemLibrary.LineTraceSingle` _worldlocation (+ _worldlocation (* _worlddirection 10000.0)) "TraceTypeQuery1"))
    (if _returnvalue
      (bind _asbp_ship (cast `/Game/SeaBattle/Dev/Core/BP_Ship` (`.HitActor` (`GameplayStatics.BreakHitResult` _outhit))))
      (bind _mainmanager (`self.MainManager`)
        (:`then`
          (bind (_issuccessful _lastcoord) (`/Game/SeaBattle/Dev/Core/BP_GameManager.PullOutShip` _mainmanager _asbp_ship))
          (if _issuccessful
            (`|ExecutionSequence`
              (:`then_0`
                (set `self.LastCellID` _lastcoord))
              (:`then_1`
                (`self.SetShipPlacingMode`))
              (:`then_2`
                (bind _returnvalue_2 (`KismetSystemLibrary.K2_SetTimerDelegate` (`|CreateDelegate` :!event `OnMousePositionChange`) 0.01 true true))
                (set `self.MouseFollowTimer` _returnvalue_2)))))
        (:`else`
          (`KismetSystemLibrary.PrintString` "Error: GameManager is not valid. (BP_MainPlayerController | IA_RemoveShip)"))))))

(event `EnhancedInput|/Game/SeaBattle/Dev/Input/Actions/IA_RotateShip`
  (params (ActionValue :type Boolean) (ElapsedSeconds :type "Float (double-precision)") (TriggeredSeconds :type "Float (double-precision)") (InputAction :type "InputAction Object Reference" :default "/Game/SeaBattle/Dev/Input/Actions/IA_RotateShip.IA_RotateShip"))
  (bind _currentshipptr (`/Game/SeaBattle/Dev/Core/BP_GameManager.GetCurrentShip` (`self.MainManager`)))
  (:`Completed`
    (if (not (`Ship.IsPlaced` _currentshipptr))
      (`|ExecutionSequence`
        (:`then_0`
          (`/Game/SeaBattle/Dev/Core/BP_GameManager.UncolorizeAroundShip` (`self.MainManager`) (`self.LastCellID`)))
        (:`then_1`
          (`Ship.SetShipDirection` (`/Game/SeaBattle/Dev/Core/BP_GameManager.GetCurrentShip` (`self.MainManager`)) (cast `EShipDirection` (`KismetMathLibrary.Conv_IntToByte` (mod (+ (`KismetMathLibrary.Conv_ByteToInt` (`Ship.GetShipDirection` _currentshipptr)) 1) 4)))))
        (:`then_2`
          (`/Game/SeaBattle/Dev/Core/BP_GameManager.ColorizeAroundShip` (`self.MainManager`) (`self.LastCellID`)))))))

(event `EnhancedInput|/Game/SeaBattle/Dev/Input/Actions/IA_DestroyShip`
  (params (ActionValue :type Boolean) (ElapsedSeconds :type "Float (double-precision)") (TriggeredSeconds :type "Float (double-precision)") (InputAction :type "InputAction Object Reference" :default "/Game/SeaBattle/Dev/Input/Actions/IA_DestroyShip.IA_DestroyShip"))
  (:`Completed`
    (`|ExecutionSequence`
      (:`then_0`
        (`/Game/SeaBattle/Dev/Core/BP_GameManager.UncolorizeAroundShip` (`self.MainManager`) (`self.LastCellID`)))
      (:`then_1`
        (`KismetSystemLibrary.K2_ClearAndInvalidateTimerHandle` (`self.MouseFollowTimer`)))
      (:`then_2`
        (`/Game/SeaBattle/Dev/Core/BP_GameManager.DeleteShip` (`self.MainManager`)))
      (:`then_3`
        (`self.SetShipEditingMode`)))))

(fn `GetRefs`
  (`|ExecutionSequence`
    (:`then_0`
      (bind _asbp_main_gamemode (cast `/Game/SeaBattle/Dev/Common/BP_MainGamemode` (`GameplayStatics.GetGameMode`)))
      (set `self.As BP Main Gamemode` _asbp_main_gamemode))
    (:`then_1`
      (bind _returnvalue (`|SpawnActorFromClass` "/Game/SeaBattle/Dev/Core/BP_GameManager.BP_GameManager_C" (`KismetMathLibrary.MakeTransform` (0.0 0.0 0.0)) "Undefined" "MultiplyWithRoot" null null))
      (set `self.MainManager` _returnvalue))
    (:`then_2`
      (set `self.HUDWidget` (`/Game/SeaBattle/Dev/Core/BP_GameManager.GetHUD` (`self.MainManager`))))))

(fn `MoveShipToMouse`
  (bind (_locationx _locationy) (`self.GetMousePosition`))
  (bind (_worldlocation _worlddirection) (`self.DeprojectScreenPositionToWorld` _locationx _locationy))
  (bind (_outhit _returnvalue) (`KismetSystemLibrary.LineTraceSingle` _worldlocation (+ _worldlocation (* _worlddirection 10000.0)) "TraceTypeQuery1" false (`|MakeArray` (`/Game/SeaBattle/Dev/Core/BP_GameManager.GetCurrentShip` (`self.MainManager`)) :!type "Actor Object Reference")))
  (if _returnvalue
    (bind (_bblockinghit _binitialoverlap _time _distance _location _impactpoint _normal _impactnormal _physmat _hitactor) (`GameplayStatics.BreakHitResult` _outhit))
    (bind _asbp_sea_cell (cast `/Game/SeaBattle/Dev/Core/BP_SeaCell` _hitactor))
    (`|ExecutionSequence`
      (:`then_0`
        (bind _returnvalue_2 (`SeaCell.GetID` _asbp_sea_cell))
        (if (!= _returnvalue_2 (`self.LastCellID`))
          (`/Game/SeaBattle/Dev/Core/BP_GameManager.UncolorizeAroundShip` (`self.MainManager`) (`self.LastCellID`))
          (bind _output_get (set `self.LastCellID` _returnvalue_2))
          (`/Game/SeaBattle/Dev/Core/BP_GameManager.ColorizeAroundShip` (`self.MainManager`) _output_get)))
      (:`then_1`
        (bind (_returnvalue_x _returnvalue_y) (`KismetMathLibrary.BreakVector` (`self.K2_GetActorLocation` _hitactor)))
        (`/Game/SeaBattle/Dev/Core/BP_Ship.PlaceSmoothly` (`/Game/SeaBattle/Dev/Core/BP_GameManager.GetCurrentShip` (`self.MainManager`)) (`KismetMathLibrary.MakeVector` _returnvalue_x _returnvalue_y 500.0))))))

(fn `SetShipEditingMode`
  (`|ExecutionSequence`
    (:`then_0`
      (`EnhancedInputSubsystemInterface.AddMappingContext` (pcsubsystem `EnhancedInputLocalPlayerSubsystem` self) "/Game/SeaBattle/Dev/Input/IMC_ShipEditing.IMC_ShipEditing" 0 (struct)))
    (:`then_1`
      (`EnhancedInputSubsystemInterface.RemoveMappingContext` (pcsubsystem `EnhancedInputLocalPlayerSubsystem` self) "/Game/SeaBattle/Dev/Input/IMC_ShipPlacing.IMC_ShipPlacing" (struct)))))

(fn `SetShipPlacingMode`
  (`|ExecutionSequence`
    (:`then_0`
      (`EnhancedInputSubsystemInterface.AddMappingContext` (pcsubsystem `EnhancedInputLocalPlayerSubsystem` self) "/Game/SeaBattle/Dev/Input/IMC_ShipPlacing.IMC_ShipPlacing" 0 (struct)))
    (:`then_1`
      (`EnhancedInputSubsystemInterface.RemoveMappingContext` (pcsubsystem `EnhancedInputLocalPlayerSubsystem` self) "/Game/SeaBattle/Dev/Input/IMC_ShipEditing.IMC_ShipEditing" (struct)))))

(fn `StartInitialize`
  (bind _returnvalue (`GameplayStatics.GetPlayerController` 0))
  (bind _hudwidget (`self.HUDWidget`))
  (`|ExecutionSequence`
    (:`then_0`
      (`self.GetRefs`))
    (:`then_1`
      (`WidgetBlueprintLibrary.SetInputMode_GameAndUIEx` _returnvalue null "DoNotLock" false)
      (set `PlayerController.bShowMouseCursor` true _returnvalue))
    (:`then_2`
      (add `/Game/SeaBattle/Dev/UI/GameHUD/WBP_MainHUD.SizeButtonClicked` _hudwidget (`|CreateDelegate` :!event `OnSizeClicked`))
      (`UserWidget.AddToViewport` _hudwidget 0))))

(fn `UserConstructionScript`)