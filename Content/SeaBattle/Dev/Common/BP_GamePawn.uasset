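; Camera pawn for the SeaBattle game, providing spring-arm orbit and zoom plus a scripted camera move tied to the HUD's start click.
; Rotate input turns the arm, with pitch held between limits on input and on Tick.
; Zoom input drives a looping timer that interpolates arm length toward a clamped target.
; The start move pauses zoom and runs a timer easing location, rotation and arm length to a fixed view.
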(event `self.ReceiveTick`
  (params (DeltaSeconds :type "Float (single-precision)"))
  (bind _rotationmax (`self.RotationMax`))
  (bind _rotationmin (`self.RotationMin`))
  (bind (_relativerotation_roll _relativerotation_pitch _relativerotation_yaw) (`KismetMathLibrary.BreakRotator` (`SceneComponent.RelativeRotation` (`self.SpringArm`))))
  (bind (_relativerotation_roll_2 _relativerotation_pitch_2) (`KismetMathLibrary.BreakRotator` (`SceneComponent.RelativeRotation` (`self.SpringArm`))))
  (`SceneComponent.K2_SetRelativeRotation` (`self.SpringArm`) (`KismetMathLibrary.MakeRotator` 0.0 (`KismetMathLibrary.SelectFloat` _rotationmax (`KismetMathLibrary.SelectFloat` _rotationmin _relativerotation_pitch_2 (< _relativerotation_pitch_2 _rotationmin)) (> _relativerotation_pitch_2 _rotationmax)) _relativerotation_yaw) false false))

(event `self.ReceiveBeginPlay`
  (`|ExecutionSequence`
    (:`then_0`
      (bind _returnvalue (`KismetSystemLibrary.K2_SetTimerDelegate` (`|CreateDelegate` :!event `ZoomProcessTick`) 0.01 true true))
      (bind _output_get (set `self.ZoomProcessTimer` _returnvalue))
      (`KismetSystemLibrary.K2_PauseTimerHandle` _output_get))
    (:`then_1`
      (bind _asbp_main_player_controller (cast `/Game/SeaBattle/Dev/Common/BP_MainPlayerController` (`GameplayStatics.GetPlayerController` 0)))
      (add `/Game/SeaBattle/Dev/UI/GameHUD/WBP_MainHUD.OnStartClicked` (`/Game/SeaBattle/Dev/Common/BP_MainPlayerController.HUDWidget` _asbp_main_player_controller) (`|CreateDelegate` :!event `startmove`)))))

(event `startmove`
  (`KismetSystemLibrary.K2_PauseTimerHandle` (`self.ZoomProcessTimer`))
  (bind _returnvalue (`KismetSystemLibrary.K2_SetTimerDelegate` (`|CreateDelegate` :!event `move`) 0.01 true true))
  (set `self.NewVar` _returnvalue))

(event `EnhancedInput|/Game/SeaBattle/Dev/Input/Actions/IA_RotateCamera`
  (params (ActionValue :type "Vector2D Structure") (ElapsedSeconds :type "Float (double-precision)") (TriggeredSeconds :type "Float (double-precision)") (InputAction :type "InputAction Object Reference" :default "/Game/SeaBattle/Dev/Input/Actions/IA_RotateCamera.IA_RotateCamera"))
  (bind (_relativerotation_roll _relativerotation_pitch) (`KismetMathLibrary.BreakRotator` (`SceneComponent.RelativeRotation` (`self.SpringArm`))))
  (:`Triggered`
    (`SceneComponent.K2_AddRelativeRotation` (`self.SpringArm`) (`KismetMathLibrary.MakeRotator` 0.0 (`KismetMathLibrary.SelectFloat` 0.0 ActionValue_Y (or (and (> _relativerotation_pitch (`self.RotationMax`)) (> ActionValue_Y 0.0)) (and (< _relativerotation_pitch (`self.RotationMin`)) (< ActionValue_Y 0.0)))) ActionValue_X) false false)))

(event `EnhancedInput|/Game/SeaBattle/Dev/Input/Actions/IA_ZoomToField`
  (params (ActionValue :type "Float (double-precision)") (ElapsedSeconds :type "Float (double-precision)") (TriggeredSeconds :type "Float (double-precision)") (InputAction :type "InputAction Object Reference" :default "/Game/SeaBattle/Dev/Input/Actions/IA_ZoomToField.IA_ZoomToField"))
  (:`Triggered`
    (set `self.ZoomDir` ActionValue)
    (`|ExecutionSequence`
      (:`then_0`
        (set `self.ZoomTarget` (`SpringArmComponent.TargetArmLength` (`self.SpringArm`))))
      (:`then_1`
        (`KismetSystemLibrary.K2_UnPauseTimerHandle` (`self.ZoomProcessTimer`))))))

(event `ZoomProcessTick`
  (`|ExecutionSequence`
    (:`then_0`
      (set `self.ZoomTarget` (`KismetMathLibrary.FClamp` (+ (`self.ZoomTarget`) (* (`self.ZoomDir`) 500.0)) (`self.ZoomMin`) (`self.ZoomMax`))))
    (:`then_1`
      (set `SpringArmComponent.TargetArmLength` (`KismetMathLibrary.FInterpTo` (`SpringArmComponent.TargetArmLength` (`self.SpringArm`)) (`self.ZoomTarget`) (`GameplayStatics.GetWorldDeltaSeconds`) (`self.ZoomSpeed`)) (`self.SpringArm`)))
    (:`then_2`
      (if (`KismetMathLibrary.NearlyEqual_FloatFloat` (`SpringArmComponent.TargetArmLength` (`self.SpringArm`)) (`self.ZoomTarget`) 0.1)
        (set `SpringArmComponent.TargetArmLength` (`self.ZoomTarget`) (`self.SpringArm`))
        (`KismetSystemLibrary.K2_UnPauseTimerHandle` (`self.ZoomProcessTimer`))
        (else
          (set `self.ZoomDir` 0.0))))))

(fn `move`
  (set `self.alpha` (+ (`self.alpha`) 0.005))
  (`self.K2_SetActorLocation` (`|EaseFunction` "EaseOut" (`self.alpha`) (`self.K2_GetActorLocation`) (-3100.0 0.0 0.0) 0.03) false true)
  (`SceneComponent.K2_SetRelativeRotation` (`self.SpringArm`) (`|EaseFunction` "EaseOut" (`self.alpha`) (`SceneComponent.RelativeRotation` (`self.SpringArm`)) (struct :`Pitch` -40.0) true 0.03) false false)
  (set `SpringArmComponent.TargetArmLength` (`|EaseFunction` "EaseOut" (`self.alpha`) (`SpringArmComponent.TargetArmLength` (`self.SpringArm`)) 8000.0 0.03) (`self.SpringArm`))
  (if (`KismetMathLibrary.NearlyEqual_FloatFloat` (`self.alpha`) 1.0)
    (set `self.alpha` 0.0)
    (`KismetSystemLibrary.K2_ClearAndInvalidateTimerHandle` (`self.NewVar`))))

(fn `UserConstructionScript`)