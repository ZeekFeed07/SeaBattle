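; Game manager for a Sea Battle game that runs the ship setup phase on the player's field.
; On BeginPlay it spawns player and enemy BP_SeaFields and creates the HUD, whose size buttons spawn ships from a per-size stock.
; Placing, moving and pulling out ships are delegated to the field and ship, gated by controller-to-field ownership checks.
; The HUD's start click eases the lowered enemy field up into view on a looping timer.
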(event `self.ReceiveBeginPlay`
  (`|ExecutionSequence`
    (:`then_0`
      (`self.StartInitialize`))))

(event `OnSizeButtonClicked`
  (params (`Ship Size` :type "EShipLength Enum" :default "ONE"))
  (bind (_value _returnvalue) (`BlueprintMapLibrary.Map_Find` (`self.ShipsCount`) `Ship Size`))
  (if _returnvalue
    (if (> _value 0)
      (`BlueprintMapLibrary.Map_Add` (`self.ShipsCount`) `Ship Size` (- _value 1))
      (`self.DeleteShip`)
      (`self.CreateShip` `Ship Size`)
      (if (== (`BlueprintMapLibrary.Map_Find` (`self.ShipsCount`) `Ship Size`) 0)
        (`/Game/SeaBattle/Dev/UI/GameHUD/WBP_MainHUD.UpdateButtonState` (`self.PlayerHUD`) `Ship Size` false)))))

(event `OnStartClicked`
  (`self.AnimateEnemyField`))

(fn `AnimateEnemyField`
  (if (not (`KismetMathLibrary.EqualExactly_VectorVector` (`self.K2_GetActorLocation` (`self.EnemyField`)) (-6200.0 0.0 0.0)))
    (bind _returnvalue (`KismetSystemLibrary.K2_SetTimerDelegate` (`|CreateDelegate` :!event `AnimateEnemyFieldProcess`) 0.01 true true))
    (set `self.AnimateEnemyFieldTimer` _returnvalue)))

(fn `AnimateEnemyFieldProcess`
  (set `self.FieldAnimateAlpha` (+ (`self.FieldAnimateAlpha`) 0.001))
  (`SeaField.SetActorLocation` (`self.EnemyField`) (`|EaseFunction` "EaseIn" (`self.FieldAnimateAlpha`) (`self.K2_GetActorLocation` (`self.EnemyField`)) (-6200.0 0.0 0.0)))
  (if (`KismetMathLibrary.NearlyEqual_FloatFloat` (`self.FieldAnimateAlpha`) 1.0 0.001)
    (`SeaField.SetActorLocation` (`self.EnemyField`) (-6200.0 0.0 0.0))
    (set `self.FieldAnimateAlpha` 0.0)
    (`KismetSystemLibrary.K2_ClearAndInvalidateTimerHandle` (`self.AnimateEnemyFieldTimer`))))

(fn `CreateShip`
  (params (Size :type "EShipLength Enum" :default "ONE"))
  (bind _returnvalue (`|SpawnActorFromClass` "/Game/SeaBattle/Dev/Core/BP_Ship.BP_Ship_C" (`KismetMathLibrary.MakeTransform` (0.0 0.0 500.0)) "Undefined" "MultiplyWithRoot" null null))
  (`Ship.SetShipLength` _returnvalue Size)
  (set `self.CurrentShipPtr` _returnvalue)
  (return))

(fn `DeleteShip`
  (bind _shipscount (`self.ShipsCount`))
  (bind _currentshipptr (`self.CurrentShipPtr`)
    (:`then`
      (bind _returnvalue (`Ship.GetShipLength` _currentshipptr))
      (bind (_value _returnvalue_2) (`BlueprintMapLibrary.Map_Find` _shipscount _returnvalue))
      (if _returnvalue_2
        (if (== _value 0)
          (`/Game/SeaBattle/Dev/UI/GameHUD/WBP_MainHUD.UpdateButtonState` (`self.PlayerHUD`) _returnvalue true))
        (`BlueprintMapLibrary.Map_Add` _shipscount _returnvalue (+ _value 1))
        (`self.K2_DestroyActor` _currentshipptr)
        (set `self.CurrentShipPtr` null :!label _label)
        (return)))
    (:`else`
      (goto _label))))

(fn `GetCurrentShip`
  (returns (CurrentShipPtr :type "/Game/SeaBattle/Dev/Core/BP_Ship Object Reference"))
  (return (`self.CurrentShipPtr`)))

(fn `GetHUD`
  (returns (PlayerHUD :type "/Game/SeaBattle/Dev/UI/GameHUD/WBP_MainHUD Object Reference"))
  (return (`self.PlayerHUD`)))

(fn `GetPlayerFieldOwner`
  (returns (`Controller Ref` :type "PlayerController Object Reference"))
  (bind _output_controllerref (break `/Game/SeaBattle/Dev/Core/S_FieldOwningPair` (`|GetArrayItem` (`self.Owners`))))
  (bind _asplayer_controller (cast `PlayerController` _output_controllerref))
  (return _asplayer_controller))

(fn `IsOwnField`
  (params (Pair :type "/Game/SeaBattle/Dev/Core/S_FieldOwningPair Structure"))
  (returns (out :type Boolean))
  (bind (_pair_controllerref _pair_fieldref) (break `/Game/SeaBattle/Dev/Core/S_FieldOwningPair` (`local.Pair`)))
  (for _array_element (`self.Owners`)
    (if (and (== (break `/Game/SeaBattle/Dev/Core/S_FieldOwningPair` _array_element) _pair_controllerref) (== (`.FieldRef_5_BB524E534AA46F8FE09F52B74DEF74CC` (break `/Game/SeaBattle/Dev/Core/S_FieldOwningPair` _array_element)) _pair_fieldref))
      (return true)))
  (return false))

(fn `MoveShip`
  (params (CellPtr :type "/Game/SeaBattle/Dev/Core/BP_SeaCell Object Reference") (Caller :type "Controller Object Reference"))
  (bind _asbp_sea_field (cast `/Game/SeaBattle/Dev/Core/BP_SeaField` (`SeaCell.GetParentField` CellPtr)))
  (if (`self.IsOwnField` (make `/Game/SeaBattle/Dev/Core/S_FieldOwningPair` Caller _asbp_sea_field))
    (`/Game/SeaBattle/Dev/Core/BP_Ship.PlaceSmoothly` (`self.GetCurrentShip`) (`self.K2_GetActorLocation` CellPtr))
    (return)))

(fn `PlaceShipToField`
  (params (CellPtr :type "/Game/SeaBattle/Dev/Core/BP_SeaCell Object Reference") (Caller :type "Controller Object Reference"))
  (returns (IsSuccessful :type Boolean))
  (bind _currentshipptr (`self.CurrentShipPtr`))
  (bind (_returnvalue_x _returnvalue_y) (break `IntPoint` (`SeaCell.GetID` (`local.CellPtr`))))
  (`/Engine/EditorBlueprintResources/StandardMacros.IsValid` CellPtr
    (:`Is Valid`
      (bind _asbp_sea_field (cast `/Game/SeaBattle/Dev/Core/BP_SeaField` (`SeaCell.GetParentField` CellPtr))
        (:`then`
          (if (`self.IsOwnField` (make `/Game/SeaBattle/Dev/Core/S_FieldOwningPair` Caller _asbp_sea_field))
            (`self.PlayerField`
              (:`then`
                (bind _returnvalue (`SeaField.AddShip` (`self.PlayerField`) _currentshipptr _returnvalue_x _returnvalue_y (`Ship.GetShipDirection` _currentshipptr)))
                (if _returnvalue
                  (`/Game/SeaBattle/Dev/Core/BP_Ship.PlaceSmoothly` (`self.CurrentShipPtr`) (`self.K2_GetActorLocation` (`local.CellPtr`)))
                  (set `self.CurrentShipPtr` null)
                  (return true)
                  (else
                    _)))
              (:`else`
                (`KismetSystemLibrary.PrintString` "Error: Field is not valid. (BP_GameManager | PlaceShipToField)")))))
        (:`CastFailed`
          _)))
    (:`Is Not Valid`
      (`KismetSystemLibrary.PrintString` "Error: Field is not valid. (BP_GameManager | PlaceShipToField)")))
  (return false))

(fn `PullOutShip`
  (params (ShipPtr :type "/Game/SeaBattle/Dev/Core/BP_Ship Object Reference"))
  (returns (IsSuccessful :type Boolean) (LastCell :type "/Game/SeaBattle/Dev/Core/BP_SeaCell Object Reference"))
  (locals (ProbablyShipPlacedCell :type "/Game/SeaBattle/Dev/Core/BP_SeaCell Object Reference"))
  (bind _probablyshipplacedcell (`local.ProbablyShipPlacedCell`))
  (bind (_returnvalue_x _returnvalue_y) (`KismetMathLibrary.BreakVector` (`self.K2_GetActorLocation` (`self.CurrentShipPtr`))))
  (bind _output_controllerref (break `/Game/SeaBattle/Dev/Core/S_FieldOwningPair` (`|GetArrayItem` (`self.Owners`))))
  (bind _asbp_sea_cell (cast `/Game/SeaBattle/Dev/Core/BP_SeaCell` (`SeaField.GetShipPlacedCell` (`self.PlayerField`) ShipPtr)))
  (set `local.ProbablyShipPlacedCell` _asbp_sea_cell)
  (bind _returnvalue (`SeaField.RemoveShip` (`self.PlayerField`) ShipPtr))
  (if _returnvalue
    (bind _output_get (set `self.CurrentShipPtr` ShipPtr))
    (`/Game/SeaBattle/Dev/Core/BP_Ship.PlaceSmoothly` _output_get (`KismetMathLibrary.MakeVector` _returnvalue_x _returnvalue_y))
    (`self.UpdateColorAroundShip` _probablyshipplacedcell _output_controllerref))
  (return _returnvalue _probablyshipplacedcell))

(fn `SetPlayerFieldOwner`
  (params (`Controller Ref` :type "PlayerController Object Reference"))
  (`KismetArrayLibrary.Array_Set` (`self.Owners`) 0 (make `/Game/SeaBattle/Dev/Core/S_FieldOwningPair` `Controller Ref` (`self.PlayerField`)))
  (return))

(fn `StartInitialize`
  (`|ExecutionSequence`
    (:`then_0`
      (`KismetArrayLibrary.Array_Resize` (`self.Owners`) 2))
    (:`then_1`
      (bind _returnvalue (`|SpawnActorFromClass` "/Game/SeaBattle/Dev/Core/BP_SeaField.BP_SeaField_C" (`KismetMathLibrary.MakeTransform` (0.0 0.0 0.0) (struct :`Pitch` -90.0)) "Undefined" "MultiplyWithRoot" null "/Game/SeaBattle/Dev/Core/BP_SeaCell.BP_SeaCell_C" null))
      (set `self.PlayerField` _returnvalue))
    (:`then_2`
      (bind _returnvalue_2 (`|SpawnActorFromClass` "/Game/SeaBattle/Dev/Core/BP_SeaField.BP_SeaField_C" (`KismetMathLibrary.MakeTransform` (-6200.0 0.0 -1100.0) (struct :`Pitch` -90.0)) "Undefined" "MultiplyWithRoot" null "/Game/SeaBattle/Dev/Core/BP_SeaCell.BP_SeaCell_C" null))
      (set `self.EnemyField` _returnvalue_2))
    (:`then_3`
      (bind _returnvalue_3 (`|CreateWidget` "/Game/SeaBattle/Dev/UI/GameHUD/WBP_MainHUD.WBP_MainHUD_C"))
      (bind _output_get (set `self.PlayerHUD` _returnvalue_3))
      (add `/Game/SeaBattle/Dev/UI/GameHUD/WBP_MainHUD.SizeButtonClicked` _output_get (`|CreateDelegate` :!event `OnSizeButtonClicked`))
      (add `/Game/SeaBattle/Dev/UI/GameHUD/WBP_MainHUD.OnStartClicked` _output_get (`|CreateDelegate` :!event `OnStartClicked`)))))

(fn `UpdateColorAroundShip`
  (params (CellPtr :type "/Game/SeaBattle/Dev/Core/BP_SeaCell Object Reference") (Caller :type "Controller Object Reference") (Clear :type Boolean))
  (bind (_returnvalue_x _returnvalue_y) (break `IntPoint` (`SeaCell.GetID` (`local.CellPtr`))))
  (bind (_returnvalue_x_2 _returnvalue_y_2) (break `IntPoint` (`SeaCell.GetID` (`local.CellPtr`))))
  (`/Engine/EditorBlueprintResources/StandardMacros.IsValid` CellPtr
    (:`Is Valid`
      (`/Engine/EditorBlueprintResources/StandardMacros.IsValid` Caller
        (:`Is Valid`
          (bind _asbp_sea_field (cast `/Game/SeaBattle/Dev/Core/BP_SeaField` (`SeaCell.GetParentField` CellPtr)))
          (if (and (`self.IsOwnField` (make `/Game/SeaBattle/Dev/Core/S_FieldOwningPair` Caller _asbp_sea_field)) (`KismetSystemLibrary.IsValid` (`local.CellPtr`)))
            (if (`local.Clear`)
              (`SeaField.UncolorizeArea` (`self.PlayerField`) (`self.CurrentShipPtr`) _returnvalue_x _returnvalue_y)
              (else
                (`SeaField.ColorizeArea` (`self.PlayerField`) (`self.CurrentShipPtr`) _returnvalue_x_2 _returnvalue_y_2)))
            (return)))))))

(fn `UserConstructionScript`)