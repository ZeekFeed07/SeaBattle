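; BP_Ship is a ship actor for the Sea Battle game, with its body mesh and offset set by ship length.
; Direction changes rotate it 90 degrees, and hovering instantly raises or lowers the actor.
; PlaceSmoothly stores a target and unpauses a looping timer created paused at BeginPlay, avoiding Event Tick.
; The timer interpolates the ship toward the target, then snaps, pauses and resets the target to a far-off sentinel.
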(event `self.ReceiveBeginPlay`
  (bind _returnvalue (`KismetSystemLibrary.K2_SetTimerDelegate` (`|CreateDelegate` :!event `SmoothMovementTick`) 0.01 true true))
  (bind _output_get (set `self.SmoothMovementTickTimer` _returnvalue))
  (`KismetSystemLibrary.K2_PauseTimerHandle` _output_get))

(event `self.OnLengthChanged`
  (`|ExecutionSequence`
    (:`then_0`
      (`StaticMeshComponent.SetStaticMesh` (`self.Body`) (select `byte` (`self.GetShipLength`) :`0` "/Game/SeaBattle/Art/Meshes/SM_Ship_1.SM_Ship_1" :`1` "/Game/SeaBattle/Art/Meshes/SM_Ship_2.SM_Ship_2" :`2` "/Game/SeaBattle/Art/Meshes/SM_Ship_3.SM_Ship_3" :`3` "/Game/SeaBattle/Art/Meshes/SM_Ship_4.SM_Ship_4" :!type "StaticMesh Object Reference")))
    (:`then_1`
      (`SceneComponent.K2_AddWorldOffset` (`self.Body`) (`KismetMathLibrary.MakeVector` 0.0 (* (`KismetMathLibrary.Conv_ByteToInt` (`self.GetShipLength`)) 250.0)) false true))))

(event `self.OnDirectionChanged`
  (`SceneComponent.K2_AddWorldRotation` (`self.Scene`) (struct :`Yaw` 90.0) false false))

(event `OnActorHovered`
  (`self.ActorUpAnimate`))

(event `OnActorUnhovered`
  (`self.ActorDownAnimate`))

(event `PlaceSmoothly`
  (params (Target :type "Vector Structure"))
  (if (!= Target (`self.TargetToMove`) :`ErrorTolerance` 0.01)
    (set `self.TargetToMove` Target)
    (`KismetSystemLibrary.K2_UnPauseTimerHandle` (`self.SmoothMovementTickTimer`))))

(event `SmoothMovementTick`
  (`|ExecutionSequence`
    (:`then_0`
      (`self.K2_SetActorLocation` (`KismetMathLibrary.VInterpTo` (`self.K2_GetActorLocation`) (`self.TargetToMove`) (`GameplayStatics.GetWorldDeltaSeconds`) 3.0) false true))
    (:`then_1`
      (if (`KismetMathLibrary.Vector_IsNearlyZero` (- (`self.K2_GetActorLocation`) (`self.TargetToMove`)) 0.01)
        (`|ExecutionSequence`
          (:`then_0`
            (`self.K2_SetActorLocation` (`self.TargetToMove`) false true))
          (:`then_1`
            (`KismetSystemLibrary.K2_PauseTimerHandle` (`self.SmoothMovementTickTimer`)))
          (:`then_2`
            (set `self.TargetToMove` (-100000.0 -100000.0 -100000.0))))))))

(fn `ActorDownAnimate`
  (`self.K2_SetActorLocation` (- (`self.K2_GetActorLocation`) (0.0 0.0 200.0)) false true))

(fn `ActorUpAnimate`
  (`self.K2_SetActorLocation` (+ (`self.K2_GetActorLocation`) (0.0 0.0 200.0)) false true))

(fn `UserConstructionScript`)