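; Game mode for a Battleship-style game that sets up the player and enemy sea fields and enters the Preparation state on BeginPlay.
; It spawns and initializes both BP_SeaField grids, passing only the player's to the main player controller.
; Controller-requested ships spawn attached to the mouse, then decrement a per-size count map, whose result does not gate spawning.
; AddShip and the state switch are empty stubs.
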(event `self.ReceiveBeginPlay`
  ;[0 0 0 1 30] BeginPlay
  (`self.GetRefs`)
  (`self.GenerateFields`)
  (`self.SetPlayState` "NewEnumerator0"))

(event `GetRefs`
  ;[0 0 0 1 30] Getting references
  (`|ExecutionSequence`
    (:`then_0`
      (bind _asbp_main_player_controller (cast `/Game/Blueprints/BP_MainPlayerController` (`GameplayStatics.GetPlayerController` 0))
        (:`then`
          (bind _output_get (set `self.BP Main Player Controller` _asbp_main_player_controller))
          (add `/Game/Blueprints/BP_MainPlayerController.CreateShip` _output_get (`|CreateDelegate` :!event `CreatingShip`)))
        (:`CastFailed`
          (`KismetSystemLibrary.PrintString` "Error: Cast to BP_MainPlayerController failed. (BP_MainGamemode | GetRefs)"))))))

(event `CreatingShip`
  (params (Size :type Integer))
  (`|ExecutionSequence`
    (:`then_0`
      (bind _returnvalue (`|SpawnActorFromClass` "/Game/Blueprints/BP_Ship.BP_Ship_C" (`KismetMathLibrary.MakeTransform` (`self.ShipSpawnStart`)) "Undefined" "MultiplyWithRoot" null Size null))
      (`/Game/Blueprints/BP_MainPlayerController.AttachShipToMouse` (`self.BP Main Player Controller`) _returnvalue))
    (:`then_1`
      (`self.ReduceShip` Size))))

(fn `AddShip`)

(fn `GenerateFields`
  (`|ExecutionSequence`
    (:`then_0`
      (bind _returnvalue (`|SpawnActorFromClass` "/Game/Blueprints/BP_SeaField.BP_SeaField_C" (`KismetMathLibrary.MakeTransform` (`self.PlayerFieldLoc`)) "Undefined" "MultiplyWithRoot" null null))
      (bind _output_get (set `self.PlayerField` _returnvalue))
      (`|ExecutionSequence`
        (:`then_0`
          (set `SeaField.CellClass` (`self.Player Cell Class`) _output_get))
        (:`then_1`
          (set `SeaField.CellGap` (`self.CellGapPlayer`) _output_get))
        (:`then_2`
          (`SeaField.InitField` _output_get))
        (:`then_3`
          (`/Game/Blueprints/BP_MainPlayerController.SetField` (`self.BP Main Player Controller`) _output_get))))
    (:`then_1`
      (bind _returnvalue_2 (`|SpawnActorFromClass` "/Game/Blueprints/BP_SeaField.BP_SeaField_C" (`KismetMathLibrary.MakeTransform` (`self.EnemyFieldLoc`)) "Undefined" "MultiplyWithRoot" null null))
      (bind _output_get_2 (set `self.EnemyField` _returnvalue_2))
      (`|ExecutionSequence`
        (:`then_0`
          (set `SeaField.CellClass` (`self.Enemy Cell Class`) _output_get_2))
        (:`then_1`
          (set `SeaField.CellGap` (`self.CellGapEnemy`) _output_get_2))
        (:`then_2`
          (`SeaField.InitField` _output_get_2))))))

(fn `ReduceShip`
  (params (ShipSize :type Integer))
  (returns (IsCompleted :type Boolean))
  (bind _shipcount (`self.ShipCount`))
  (bind (_value _returnvalue) (`BlueprintMapLibrary.Map_Find` (`self.ShipCount`) ShipSize))
  (if _returnvalue
    (if (> _value 0)
      (`BlueprintMapLibrary.Map_Add` _shipcount (`local.ShipSize`) (- (`BlueprintMapLibrary.Map_Find` _shipcount (`local.ShipSize`)) 1))
      (return true)
      (else
        (`KismetSystemLibrary.PrintString` "No ship this size. (BP_MainGamemode | ReduceShip)")))
    (else
      (`KismetSystemLibrary.PrintString` "Undefined Key in ShipCount. (BP_MainGamemode | ReduceShip)")))
  (return false))

(fn `SetPlayState`
  (params (State :type "/Game/Blueprints/PlayState Enum" :default "NewEnumerator0"))
  (bind _output_get (set `self.GameStates` State))
  (switch `/Game/Blueprints/PlayState` _output_get))

(fn `UserConstructionScript`)