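; Player controller for a ship placement game that shows the game menu and drags a ship over the sea field with the mouse.
; Menu size button presses are relayed through CreateShip.
; An attached ship follows the cursor on a looping timer, using a deprojected trace and interpolation at a fixed height.
; The hit cell is checked against the field reference for rightward placement, and the result is only printed.
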(event `self.ReceiveBeginPlay`
  (bind _returnvalue (`GameplayStatics.GetPlayerController` 0))
  ;[0 0 0 1 30] BeginPlay
  (`|ExecutionSequence`
    (:`then_0`
      (`self.CreateWidgeet`))
    (:`then_1`
      (`WidgetBlueprintLibrary.SetInputMode_GameAndUIEx` _returnvalue null "DoNotLock" false)
      (set `PlayerController.bShowMouseCursor` true _returnvalue))))

(event `CreateWidgeet`
  (bind _returnvalue (`|CreateWidget` "/Game/UI/GameInteerface/WBP_GameMenu.WBP_GameMenu_C" (`GameplayStatics.GetPlayerController` 0)))
  (`UserWidget.AddToViewport` _returnvalue 0)
  (bind _output_get (set `self.WBP_GameMenu` _returnvalue))
  (add `/Game/UI/GameInteerface/WBP_GameMenu.ButtonSizePressed` _output_get (`|CreateDelegate` :!event `OnSizeButtonPressed`)))

(event `OnSizeButtonPressed`
  (params (Size :type Integer))
  (`self.CreateShip` Size))

(event `AttachShipToMouse`
  (params (Ship :type "Ship Object Reference (by ref)"))
  (set `self.Ship` Ship)
  (bind _returnvalue (`KismetSystemLibrary.K2_SetTimerDelegate` (`|CreateDelegate` :!event `RefreshShipPosition`) (`self.MouseFollowDelta`) true))
  (set `self.MouseFollowTimer` _returnvalue))

(event `RefreshShipPosition`
  (bind (_locationx _locationy) (`self.GetMousePosition`))
  (bind (_worldlocation _worlddirection) (`self.DeprojectScreenPositionToWorld` _locationx _locationy))
  (bind _returnvalue (+ _worldlocation (* _worlddirection 10000.0)))
  (`|ExecutionSequence`
    (:`then_0`
      (bind _outhit (`KismetSystemLibrary.LineTraceSingle` _worldlocation _returnvalue "TraceTypeQuery1" false (`|MakeArray` (`self.Ship`) :!type "Actor Object Reference") "ForDuration"))
      (bind (_bblockinghit _binitialoverlap _time _distance _location _impactpoint _normal _impactnormal _physmat _hitactor) (`GameplayStatics.BreakHitResult` _outhit))
      (bind (_returnvalue_x _returnvalue_y) (`KismetMathLibrary.BreakVector` (`KismetMathLibrary.VInterpTo` (`self.K2_GetActorLocation` (`self.Ship`)) (`KismetMathLibrary.SelectVector` _location _returnvalue _bblockinghit) (`GameplayStatics.GetWorldDeltaSeconds`) (`self.Interp Speed`))))
      (`self.K2_SetActorLocation` (`self.Ship`) (`KismetMathLibrary.MakeVector` _returnvalue_x _returnvalue_y 500.0) false false))
    (:`then_1`
      (bind _asbp_sea_field_cell (cast `/Game/Blueprints/BP_SeaFieldCell` _hitactor))
      (bind _returnvalue_2 (`SeaField.CheckPlace` (`self.FieldRef`) (`self.Ship`) (`SeaFieldCell.GetCoord` _asbp_sea_field_cell) "RIGHT"))
      (`KismetSystemLibrary.PrintString` (`KismetStringLibrary.Conv_BoolToString` _returnvalue_2)))))

(fn `SetField`
  (params (Reference :type "/Game/Blueprints/BP_SeaField Object Reference"))
  (set `self.FieldRef` Reference))

(fn `UserConstructionScript`)